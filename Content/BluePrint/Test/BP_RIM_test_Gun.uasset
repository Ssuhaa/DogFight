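; Test Blueprint for a gun lying on the ground that detects the player as groundwork for a pickup.
; CollisionComp overlap casts to BP_RIM_testPlayer, stores the reference and enables input on the gun for player controller 0; end overlap disables it.
; The PunchGrab pickup exists only as comments and unconnected DestroyActor nodes, alongside unreachable duplicate logic for BP_RIM_Player.
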(event `CustomEvent`
  (params (OverlappedComponent :type "PrimitiveComponent Object Reference") (OtherActor :type "Actor Object Reference") (OtherComp :type "PrimitiveComponent Object Reference") (OtherBodyIndex :type Integer) (bFromSweep :type Boolean) (SweepResult :type "HitResult Structure (by ref)"))
  ;[1 1 1 1 12] 바닥에 있는 총이 플레이어와 부딪힌다.
)

(event `self.collisionComp.OnComponentBeginOverlap`
  (params (OverlappedComponent :type "PrimitiveComponent Object Reference") (OtherActor :type "Actor Object Reference") (OtherComp :type "PrimitiveComponent Object Reference") (OtherBodyIndex :type Integer) (bFromSweep :type Boolean) (SweepResult :type "HitResult Structure (by ref)"))
  ;[1 1 1] Comment
  ;;[1 1 1 1 12] 바닥에 있는 총이 플레이어와 부딪힌다.
  (bind _asbp_rim_test_player (cast `/Game/BluePrint/Test/BP_RIM_testPlayer` OtherActor)) ; 바닥에 있는 총과 충돌할 액터의 클래스.\n[플레이어]
  (set `self.BP RIM Test Player` _asbp_rim_test_player)
  (`self.EnableInput` self (`GameplayStatics.GetPlayerController` 0)) ; 키 조작
)

(event `self.ReceiveActorBeginOverlap`
  (params (OtherActor :type "Actor Object Reference")))

(event `CustomEvent_1`
  (params (OverlappedComponent :type "PrimitiveComponent Object Reference") (OtherActor :type "Actor Object Reference") (OtherComp :type "PrimitiveComponent Object Reference") (OtherBodyIndex :type Integer)))

(event `self.collisionComp.OnComponentEndOverlap`
  (params (OverlappedComponent :type "PrimitiveComponent Object Reference") (OtherActor :type "Actor Object Reference") (OtherComp :type "PrimitiveComponent Object Reference") (OtherBodyIndex :type Integer))
  ;[1 1 1] Comment
  (cast `/Game/BluePrint/Test/BP_RIM_testPlayer` OtherActor) ; 바닥에 있는 총과 충돌할 액터의 클래스.\n[플레이어]
  (`self.DisableInput` (`GameplayStatics.GetPlayerController` 0)) ; 키 조작
)

(event `InputAction|PunchGrab`
  (params (Key :type "Key Structure"))
  ;[1 1 1 1 12] 플레이어가  PunchGrab 키를 눌렀으면
)

(event `InputAction|PunchGrab`
  (params (Key :type "Key Structure"))
  ;[1 1 1 1 12] 조건: 플레이어가  PunchGrab 키를 눌렀으면
)

(fn `UserConstructionScript`)