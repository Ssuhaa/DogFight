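; BP_RIM_Gun is a gun lying on the ground, meant to be picked up by the player, but its graph is currently inert.
; Its collision overlap events are empty, and the pickup logic sits in disconnected nodes that never run.
; Those nodes cast the overlapping actor to BP_RIM_Player, toggle input on begin and end overlap, and call VisibleGun on the player before destroying the gun.
; Comments describe a PunchGrab key trigger, but no such input event exists.
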(event `self.ReceiveActorBeginOverlap`
  (params (OtherActor :type "Actor Object Reference")))

(event `self.collisionComp.OnComponentBeginOverlap`
  (params (OverlappedComponent :type "PrimitiveComponent Object Reference") (OtherActor :type "Actor Object Reference") (OtherComp :type "PrimitiveComponent Object Reference") (OtherBodyIndex :type Integer) (bFromSweep :type Boolean) (SweepResult :type "HitResult Structure (by ref)"))
  ;[1 1 1 1 12] 바닥에 있는 총이 플레이어와 부딪힌다.
)

(event `self.collisionComp.OnComponentEndOverlap`
  (params (OverlappedComponent :type "PrimitiveComponent Object Reference") (OtherActor :type "Actor Object Reference") (OtherComp :type "PrimitiveComponent Object Reference") (OtherBodyIndex :type Integer)))

(event `InputAction|PunchGrab`
  (params (Key :type "Key Structure"))
  ;[1 1 1 1 12] 조건: 플레이어가  PunchGrab 키를 눌렀으면
)

(fn `UserConstructionScript`)